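; Enemy wave manager that starts a new wave from the level's BP_EnemySpawner actors once no BP_Enemy actors remain.
; NewEnemyWaveCheck counts living enemies and, at zero, calls SpawnNewEnemies and a SpawnActor at the passed transform with no class shown.
; SpawnNewEnemies waits a short delay, then calls SpawnNewEnemy on every spawner found.
; Progress is reported through debug print strings, including a spawner count on BeginPlay.
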(event Custom|NewEnemyWaveCheck
  (params (Transform :type Transform))
  (Development|PrintString "Checking enemy count")
  (bind _outactors (Actor|GetAllActorsOfClass "/Game/blueprints/BP_Enemy.BP_Enemy_C"))
  (if (> (Utilities|Array|Length _outactors) 0)
    (Development|PrintString "There are still more enemies in the level.")
    (else
      (CallFunction|SpawnNewEnemies)
      (Game|SpawnActorfromClass "/Game/blueprints/BP_Key.BP_Key_C" Transform "Undefined" "MultiplyWithRoot" 0 0))))

(event Custom|Spawn%20New%20Enemies
  (Development|PrintString "spawning new enemies 4 seconds" true true "(R=1.000000,G=0.011788,B=0.922670,A=1.000000)" 5.0)
  (Utilities|FlowControl|Delay 4.0)
  (bind _outactors (Actor|GetAllActorsOfClass "/Game/blueprints/BP_EnemySpawner.BP_EnemySpawner_C"))
  (for (_array_element _array_index) _outactors
    (Default|SpawnNewEnemy _array_element)
    (Development|PrintString (Utilities|String|Append (Utilities|String|ToString(Integer) _array_index) ". " (Utilities|GetDisplayName _array_element) " is spawning....") true true "(R=1.000000,G=0.000000,B=0.229848,A=1.000000)" 5.0))
  (Development|PrintString "New wave complete!"))

(event EventBeginPlay
  (Development|PrintString "SpawnManager is active.")
  (bind _outactors (Actor|GetAllActorsOfClass "/Game/blueprints/BP_EnemySpawner.BP_EnemySpawner_C"))
  (Development|PrintString (Utilities|String|Append " There are " (Utilities|String|ToString(Integer) (Utilities|Array|Length _outactors)) " spawners in the level" " There are" " ##" " enemies in the level.") true true "(R=0.000000,G=0.635417,B=0.015343,A=1.000000)" 1e+01))

(event Collision|EventActorBeginOverlap
  (params (OtherActor :type Actor%20Object%20Reference)))

(event EventTick
  (params (DeltaSeconds :type Float%20%28single-precision%29)))

(fn ConstructionScript)