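; Falling platform that drops shortly after the third-person character steps on it, then returns to its starting spot.
; A box trigger overlap, gated by a ready flag, plays an explosion sound and starts a delayed countdown before the platform simulates physics.
; After a fall delay, physics stops and a timeline lerps the platform back to its saved transform and re-arms it.
; Material swaps signal each state: active, falling, resetting and ready.
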(event OnComponentBeginOverlap(BoxTrigger)
  (params (OverlappedComponent :type Primitive%20Component%20Object%20Reference) (OtherActor :type Actor%20Object%20Reference) (OtherComp :type Primitive%20Component%20Object%20Reference) (OtherBodyIndex :type Integer) (bFromSweep :type Boolean) (SweepResult :type Hit%20Result%20Structure%20%28by%20ref%29))
  (Development|PrintString "Something is standing on me")
  (if (Variables|Default|GetisReady)
    (Utilities|Casting|CastToBP_ThirdPersonCharacter OtherActor)
    (CallFunction|Activate)))

(event Custom|Activate
  (Audio|PlaySoundatLocation "/Game/StarterContent/Audio/Explosion01.Explosion01" (Transformation|GetWorldLocation (Variables|Default|GetPlatform)) "0, 0, 0" 0.5 2.0 0.0 0 0 0 0)
  (Variables|Default|SetisReady false)
  (Development|PrintString "Starting Countdown!")
  (Rendering|Material|SetMaterial (Variables|Default|GetPlatform) 0 "/Game/LevelPrototyping/Materials/FallingPlatforms/Mi_ActivePlatform.Mi_ActivePlatform")
  (Utilities|FlowControl|Delay (Variables|PlatformSettings|GetFallDelayDuration))
  (CallFunction|Falling))

(event Custom|Falling
  (Development|PrintString "Falling!")
  (Rendering|Material|SetMaterial (Variables|Default|GetPlatform) 0 "/Game/LevelPrototyping/Materials/FallingPlatforms/Mi_FallingPlatform.Mi_FallingPlatform")
  (Physics|SetSimulatePhysics (Variables|Default|GetPlatform) true)
  (Utilities|FlowControl|Delay (Variables|PlatformSettings|GetFall%20Duration))
  (CallFunction|Reset))

(event Custom|Reset
  (Development|PrintString "Resetting the platform")
  (Rendering|Material|SetMaterial (Variables|Default|GetPlatform) 0 "/Game/LevelPrototyping/Materials/FallingPlatforms/Mi_ResettingPlatform.Mi_ResettingPlatform")
  (Physics|SetSimulatePhysics (Variables|Default|GetPlatform) false)
  (Variables|Default|SetFallenTransform (Transformation|GetWorldTransform (Variables|Default|GetPlatform)))
  (bind _newtrack_0 (Timeline|GoBackToStartTransform PlayFromStart)
    (:Update
      (Transformation|SetWorldTransform (Variables|Default|GetPlatform) (Math|Transform|Lerp(Transform) (Variables|Default|GetFallenTransform) (Variables|Default|GetStarting%20Transform) _newtrack_0) false false))
    (:Finished
      (Variables|Default|SetisReady true)
      (Rendering|Material|SetMaterial (Variables|Default|GetPlatform) 0 "/Game/LevelPrototyping/Materials/FallingPlatforms/Mi_ReadyPlatform.Mi_ReadyPlatform"))))

(event EventBeginPlay
  (Variables|Default|SetStarting%20Transform (Transformation|GetWorldTransform (Variables|Default|GetPlatform))))

(event Collision|EventActorBeginOverlap
  (params (OtherActor :type Actor%20Object%20Reference)))

(event EventTick
  (params (DeltaSeconds :type Float%20%28single-precision%29)))

(fn ConstructionScript)